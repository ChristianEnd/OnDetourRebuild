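; BP_RotatingGear is an environment prop of four gear meshes that turn with staggered starts, accompanied by FMOD audio.
; RotateMe runs on BeginPlay or via the Trigger event, using a Sequence with Delays to start one timeline per gear.
; Each timeline's Slower track drives a rotator lerp through a full turn of its gear's relative rotation.
; BeginPlay also starts three FMOD audio components in a staggered sequence.
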(event Custom|RotateMe
  ;[1 1 1] Rotate
  (Utilities|FlowControl|Sequence
    (:then_0
      (bind _slower (Timeline|Timeline Play)
        (:Update
          (Transformation|SetRelativeRotation (Variables|Default|GetGearSingleMidFree) (Math|Rotator|Lerp(Rotator) "0, 0, 0" "0.000000,0.000000,360.000000" _slower) false false))))
    (:then_1
      (Utilities|FlowControl|Delay 1.0)
      (bind _slower_2 (Timeline|Timeline_0 PlayFromStart)
        (:Update
          (Transformation|SetRelativeRotation (Variables|Default|GetGearSingleMidFree3) (Math|Rotator|Lerp(Rotator) "0, 0, 0" "0.000000,0.000000,360.000000" _slower_2) false false))))
    (:then_2
      (Utilities|FlowControl|Delay 1.35)
      (bind _slower_3 (Timeline|Timeline_1 PlayFromStart)
        (:Update
          (Transformation|SetRelativeRotation (Variables|Default|GetGearSingleMidFree1) (Math|Rotator|Lerp(Rotator) "0, 0, 0" "0.000000,0.000000,360.000000" _slower_3) false false))))
    (:then_3
      (Utilities|FlowControl|Delay 4.0)
      (bind _slower_4 (Timeline|Timeline_2 PlayFromStart)
        (:Update
          (Transformation|SetRelativeRotation (Variables|Default|GetGearSingleMidFree2) (Math|Rotator|Lerp(Rotator) "0, 0, 0" "0.000000,0.000000,360.000000" _slower_4) false false))))))

(event EventBeginPlay
  (CallFunction|RotateMe)
  (Class|FMODAudioComponent|Play (Variables|Default|GetFMODAudio))
  (Utilities|FlowControl|Delay 1.0)
  (Class|FMODAudioComponent|Play (Variables|Default|GetFMODAudio1))
  (Utilities|FlowControl|Delay 0.5)
  (Class|FMODAudioComponent|Play (Variables|Default|GetFMODAudio2)))

(event Collision|EventActorBeginOverlap
  (params (OtherActor :type Actor%20Object%20Reference)))

(event EventTrigger
  (params (On :type Boolean) (Actor :type Actor%20Object%20Reference))
  (CallFunction|RotateMe))

(fn ConstructionScript)