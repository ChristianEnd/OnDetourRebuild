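; Destructible bars Geometry Collection actor that reacts once when struck by a physics-simulating component, apparently as part of a crane cutscene.
; The first such hit has GM_Basic play the impact and stop the crane sound, plays a 2D metal sound, and calls CutRope on a target.
; Global audio parameters mute all track volume on impact, then raise VolumeHighClean after a short delay.
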(event Custom|PlayRockSizzle
  (Class|FMODBlueprintStatics|PlayEvent2D "/Game/FMOD/Events/Environment/SingleSounds/SingleMetalMultiSounds.SingleMetalMultiSounds"))

(event Custom|CallEvent01
  (Default|CutRope (Variables|Default|GetTarget)))

(event Custom|Impact%20Sound
  (bind _asgm_basic (Utilities|Casting|CastToGM_Basic (Game|GetGameMode)))
  (Default|PlayImpact _asgm_basic)
  (Default|StopCutsceneCraneSound _asgm_basic)
  (Class|FMODBlueprintStatics|SetGlobalParameterbyName "AllTrackVolume" 0.0)
  (Utilities|FlowControl|Delay 2.0)
  (Class|FMODBlueprintStatics|SetGlobalParameterbyName "VolumeHighClean" 1.0))

(event EventBeginPlay)

(event Collision|EventActorBeginOverlap
  (params (OtherActor :type Actor%20Object%20Reference)))

(event EventTick
  (params (DeltaSeconds :type Float%20%28single-precision%29)))

(event Collision|EventHit
  (params (MyComp :type Primitive%20Component%20Object%20Reference) (Other :type Actor%20Object%20Reference) (OtherComp :type Primitive%20Component%20Object%20Reference) (bSelfMoved :type Boolean) (HitLocation :type Vector :default "0, 0, 0") (HitNormal :type Vector :default "0, 0, 0") (NormalImpulse :type Vector :default "0, 0, 0") (Hit :type Hit%20Result%20Structure%20%28by%20ref%29))
  (if (Physics|IsSimulatingPhysics OtherComp "None")
    (Utilities|FlowControl|DoOnce false
      (:Completed
        (CallFunction|ImpactSound)
        (CallFunction|PlayRockSizzle)
        (CallFunction|CallEvent01)))))

(fn ConstructionScript)