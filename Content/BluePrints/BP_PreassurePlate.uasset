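; Pressure plate actor that sinks while a Character stands on it and triggers linked objects once fully pressed.
; Collision overlaps play or reverse the ButtonAnim timeline, which lerps the button down and back up.
; When the forward animation finishes, it plays the assigned level sequence and sends InteractMessage through BPI_Interactable to ActorsToTrigger.
; Releasing the plate only raises the button, without notifying those actors.
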(event OnComponentBeginOverlap(Collision)
  (params (OverlappedComponent :type Primitive%20Component%20Object%20Reference) (OtherActor :type Actor%20Object%20Reference) (OtherComp :type Primitive%20Component%20Object%20Reference) (OtherBodyIndex :type Integer) (bFromSweep :type Boolean) (SweepResult :type Hit%20Result%20Structure%20%28by%20ref%29))
  (bind _pressureplatesequence (Variables|Default|GetPressurePlateSequence))
  (bind _sequenceplayer (Variables|/Script/LevelSequence.LevelSequenceActor|GetSequencePlayer _pressureplatesequence))
  (Utilities|Casting|CastToCharacter OtherActor)
  (bind (_direction _alpha) (Timeline|ButtonAnim Play)
    (:Update
      (Transformation|SetRelativeLocation (Variables|Default|GetButton) (Math|Vector|Lerp(Vector) "0, 0, 0" "0.000000,0.000000,-25.000000" _alpha) false false))
    (:Finished
      (switch Utilities|FlowControl|Switch|SwitchonETimelineDirection _direction
        (:Forward
          (Utilities|FlowControl|Sequence
            (:then_0
              ;[0.3552 0.06771 0.06771] PlayLevelSquence
              (Utilities|IsValid _sequenceplayer
                (:Is%20Valid
                  (Sequencer|Player|Play _sequenceplayer :!class /Script/MovieScene.MovieSceneSequencePlayer))))
            (:then_1
              (for _array_element (Variables|Default|GetActorsToTrigger)
                (if (Utilities|DoesObjectImplementInterface 0 "/Game/BluePrints/Interfaces/BPI_Interactable.BPI_Interactable_C")
                  (Class|BPIInteractable|Interact(Message) _array_element (Variables|Default|GetIsActive)))))))))))

(event OnComponentEndOverlap(Collision)
  (params (OverlappedComponent :type Primitive%20Component%20Object%20Reference) (OtherActor :type Actor%20Object%20Reference) (OtherComp :type Primitive%20Component%20Object%20Reference) (OtherBodyIndex :type Integer))
  (bind _pressureplatesequence (Variables|Default|GetPressurePlateSequence))
  (bind _sequenceplayer (Variables|/Script/LevelSequence.LevelSequenceActor|GetSequencePlayer _pressureplatesequence))
  (Utilities|Casting|CastToCharacter OtherActor)
  (bind (_direction _alpha) (Timeline|ButtonAnim Reverse)
    (:Update
      (Transformation|SetRelativeLocation (Variables|Default|GetButton) (Math|Vector|Lerp(Vector) "0, 0, 0" "0.000000,0.000000,-25.000000" _alpha) false false))
    (:Finished
      (switch Utilities|FlowControl|Switch|SwitchonETimelineDirection _direction
        (:Forward
          (Utilities|FlowControl|Sequence
            (:then_0
              ;[0.3552 0.06771 0.06771] PlayLevelSquence
              (Utilities|IsValid _sequenceplayer
                (:Is%20Valid
                  (Sequencer|Player|Play _sequenceplayer :!class /Script/MovieScene.MovieSceneSequencePlayer))))
            (:then_1
              (for _array_element (Variables|Default|GetActorsToTrigger)
                (if (Utilities|DoesObjectImplementInterface 0 "/Game/BluePrints/Interfaces/BPI_Interactable.BPI_Interactable_C")
                  (Class|BPIInteractable|Interact(Message) _array_element (Variables|Default|GetIsActive)))))))))))

(event EventBeginPlay)

(event Collision|EventActorBeginOverlap
  (params (OtherActor :type Actor%20Object%20Reference)))

(event EventTick
  (params (DeltaSeconds :type Float%20%28single-precision%29)))

(fn ConstructionScript)