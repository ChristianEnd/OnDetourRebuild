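; Combination puzzle manager that tracks which actors are triggered and reacts once when they satisfy a wanted combination.
; Trigger events add or remove actors from the current list, then compare its length to the wanted list.
; On equal lengths, the first wanted element found in the current list breaks the loop and counts as success.
; Success passes a DoOnce, messages target actors through BPI_Trigger and plays a sequence.
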(event Custom|BreakLoop
  (bind _sequences (Variables|Default|GetSequences))
  (bind _sequenceplayer (Variables|/Script/LevelSequence.LevelSequenceActor|GetSequencePlayer _sequences))
  ;[1 1 1] CheckIfCombinationIsCorrect
  (Utilities|Array|ForEachLoopwithBreak (Variables|Default|GetWantedCombination)) ; enters at Break
)

(event EventTrigger
  (params (On :type Boolean) (Actor :type Actor%20Object%20Reference))
  (bind _sequences (Variables|Default|GetSequences))
  (bind _sequenceplayer (Variables|/Script/LevelSequence.LevelSequenceActor|GetSequencePlayer _sequences))
  ;[1 1 1] RemoveTriggeredObjectFromList
  (if On
    (Utilities|Array|Add (Variables|Default|GetCurrentCombination) Actor)
    (if (== (Utilities|Array|Length (Variables|Default|GetCurrentCombination)) (Utilities|Array|Length (Variables|Default|GetWantedCombination))) :!label _label
      (Variables|Default|SetIsLoopBroken false)
      ;[1 1 1] CheckIfCombinationIsCorrect
      (bind _array_element (Utilities|Array|ForEachLoopwithBreak (Variables|Default|GetWantedCombination))
        (:LoopBody
          (if (!= (Utilities|Array|FindItem (Variables|Default|GetCurrentCombination) _array_element) -1)
            ;[1 1 1] StopLoopIfMistakeFound
            (CallFunction|BreakLoop)
            (Variables|Default|SetIsLoopBroken true)))
        (:Completed
          (if (Variables|Default|GetIsLoopBroken)
            (Utilities|FlowControl|DoOnce false
              (:Completed
                (Utilities|FlowControl|Sequence
                  (:then_0
                    ;[1 1 1] ActorToTrigger
                    (for _array_element_2 (Variables|Default|GetActorsToTrigger)
                      (if (Utilities|DoesObjectImplementInterface _array_element_2 "/Game/BluePrints/Interfaces/BPI_Trigger.BPI_Trigger_C")
                        (Class|BPITrigger|Trigger(Message) _array_element_2 true self))))
                  (:then_1
                    ;[1 1 1] PlaySequence
                    (Utilities|IsValid _sequenceplayer
                      (:Is%20Valid
                        (Sequencer|Player|Play _sequenceplayer :!class /Script/MovieScene.MovieSceneSequencePlayer)))))))))))
    (elif (!= (Utilities|Array|FindItem (Variables|Default|GetCurrentCombination) Actor) -1)
      (Utilities|Array|RemoveItem (Variables|Default|GetCurrentCombination) Actor)
      (goto _label))))

(fn ConstructionScript)