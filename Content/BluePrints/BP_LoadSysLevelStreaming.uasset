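; Trigger volume that swaps streamed sublevels when the player enters it.
; On overlap by an actor implementing BPI_Player, it loads and shows the SubLevels entry selected by LevelToLoad without blocking, then unloads the LevelToUnload entry with a blocking unload.
; The construction script sizes the Collision box from the InBoxExtent variable.
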(event OnComponentBeginOverlap(Collision)
  (params (OverlappedComponent :type Primitive%20Component%20Object%20Reference) (OtherActor :type Actor%20Object%20Reference) (OtherComp :type Primitive%20Component%20Object%20Reference) (OtherBodyIndex :type Integer) (bFromSweep :type Boolean) (SweepResult :type Hit%20Result%20Structure%20%28by%20ref%29))
  (if (Utilities|DoesObjectImplementInterface OtherActor "/Game/BluePrints/Interfaces/BPI_Player.BPI_Player_C")
    (Game|LoadStreamLevel(byName) (Utilities|Array|Get(acopy) (Variables|Default|GetSubLevels) (Variables|Default|GetLevelToLoad)) true)
    (Game|UnloadStreamLevel(byName) (Utilities|Array|Get(acopy) (Variables|Default|GetSubLevels) (Variables|Default|GetLevelToUnload)) true)))

(fn ConstructionScript
  (Components|Box|SetBoxExtent (Variables|Default|GetCollision) (Variables|Default|GetIn%20Box%20Extent) true))