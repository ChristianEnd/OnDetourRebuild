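; Generic one-shot trigger actor that activates linked actors when its Collision component is overlapped by an actor implementing BPI_Trigger.
; On the first qualifying overlap it sets IsActive, prints a debug string and sends TriggerMessage to each valid Interactable that implements the same interface.
; If PlaySequence is set, it then plays the assigned LevelSequence once.
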(event OnComponentBeginOverlap(Collision)
  (params (OverlappedComponent :type Primitive%20Component%20Object%20Reference) (OtherActor :type Actor%20Object%20Reference) (OtherComp :type Primitive%20Component%20Object%20Reference) (OtherBodyIndex :type Integer) (bFromSweep :type Boolean) (SweepResult :type Hit%20Result%20Structure%20%28by%20ref%29))
  (bind _levelsequence (Variables|Default|GetLevelSequence))
  (bind _sequenceplayer (Variables|/Script/LevelSequence.LevelSequenceActor|GetSequencePlayer _levelsequence))
  (if (Utilities|DoesObjectImplementInterface OtherActor "/Game/BluePrints/Interfaces/BPI_Trigger.BPI_Trigger_C")
    (Utilities|FlowControl|DoOnce false
      (:Completed
        (Utilities|FlowControl|Sequence
          (:then_0
            (Variables|Default|SetIsActive true)
            (Development|PrintString "Hello")
            ;[0.2427 0.1562 0.2362] ActorToTriggerLoop
            (for _array_element (Variables|Default|GetInteractable)
              (Utilities|IsValid _array_element
                (:Is%20Valid
                  (if (Utilities|DoesObjectImplementInterface _array_element "/Game/BluePrints/Interfaces/BPI_Trigger.BPI_Trigger_C")
                    (Class|BPITrigger|Trigger(Message) _array_element (Variables|Default|GetIsActive) self))))))
          (:then_1
            (if (Variables|Default|GetPlaySequence)
              ;[0.3552 0.06771 0.06771] PlayLevelSquence
              (Utilities|FlowControl|DoOnce false
                (:Completed
                  (Utilities|IsValid _sequenceplayer
                    (:Is%20Valid
                      (Sequencer|Player|Play _sequenceplayer :!class /Script/MovieScene.MovieSceneSequencePlayer))))))))))))

(event EventBeginPlay)

(event EventTick
  (params (DeltaSeconds :type Float%20%28single-precision%29)))

(event Collision|EventActorBeginOverlap
  (params (OtherActor :type Actor%20Object%20Reference)))

(fn ConstructionScript)