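; Interactable lever that toggles a switch and notifies other actors of its state.
; Interacting plays or reverses a timeline sliding the switch and setting green emissive material.
; On finish it updates IsActive, messages Interactables via BPI_Trigger, and optionally plays a level sequence once or shows typewriter text while blocking player input, optionally self-destroying afterwards.
; Two overlap volumes show a billboard prompt and swap its empty/filled material for BPI_AtmoTrigger actors.
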(event OnComponentBeginOverlap(RadiusBillboard)
  (params (OverlappedComponent :type Primitive%20Component%20Object%20Reference) (OtherActor :type Actor%20Object%20Reference) (OtherComp :type Primitive%20Component%20Object%20Reference) (OtherBodyIndex :type Integer) (bFromSweep :type Boolean) (SweepResult :type Hit%20Result%20Structure%20%28by%20ref%29))
  ;[1 1 1] Billboard
  (if (Utilities|DoesObjectImplementInterface OtherActor "/Game/BluePrints/Interfaces/BPI_AtmoTrigger.BPI_AtmoTrigger_C")
    (Rendering|SetVisibility (Variables|Default|GetBillboard) true false)))

(event OnComponentEndOverlap(RadiusBillboard)
  (params (OverlappedComponent :type Primitive%20Component%20Object%20Reference) (OtherActor :type Actor%20Object%20Reference) (OtherComp :type Primitive%20Component%20Object%20Reference) (OtherBodyIndex :type Integer))
  ;[1 1 1] Billboard
  (if (Utilities|DoesObjectImplementInterface OtherActor "/Game/BluePrints/Interfaces/BPI_AtmoTrigger.BPI_AtmoTrigger_C")
    (Rendering|SetVisibility (Variables|Default|GetBillboard) false false)))

(event OnComponentBeginOverlap(BCOL)
  (params (OverlappedComponent :type Primitive%20Component%20Object%20Reference) (OtherActor :type Actor%20Object%20Reference) (OtherComp :type Primitive%20Component%20Object%20Reference) (OtherBodyIndex :type Integer) (bFromSweep :type Boolean) (SweepResult :type Hit%20Result%20Structure%20%28by%20ref%29))
  ;[1 1 1] Billboard
  (if (Utilities|DoesObjectImplementInterface OtherActor "/Game/BluePrints/Interfaces/BPI_AtmoTrigger.BPI_AtmoTrigger_C")
    (Rendering|Material|SetMaterial (Variables|Default|GetBillboard) 0 "/Game/Material/PreCel/M_BillboardLeverFilled.M_BillboardLeverFilled")))

(event OnComponentEndOverlap(BCOL)
  (params (OverlappedComponent :type Primitive%20Component%20Object%20Reference) (OtherActor :type Actor%20Object%20Reference) (OtherComp :type Primitive%20Component%20Object%20Reference) (OtherBodyIndex :type Integer))
  ;[1 1 1] Billboard
  (if (Utilities|DoesObjectImplementInterface OtherActor "/Game/BluePrints/Interfaces/BPI_AtmoTrigger.BPI_AtmoTrigger_C")
    (Rendering|Material|SetMaterial (Variables|Default|GetBillboard) 0 "/Game/Material/PreCel/M_BillboardLeverEmpty.M_BillboardLeverEmpty")))

(event Custom|Interacted
  (bind _returnvalue (Game|GetPlayerController 0))
  (bind _leversequence (Variables|Default|GetLeverSequence))
  (bind _sequenceplayer (Variables|/Script/LevelSequence.LevelSequenceActor|GetSequencePlayer _leversequence))
  ;[0.301 0.301 0.301] Animation Lever
  (if (not (Variables|Default|GetIsActive))
    (bind (_direction _alpha) (Timeline|LeverAnim Play)
      (:Update
        (Transformation|SetRelativeLocation (Variables|Default|GetSwitchButtonCombo_Button1) (Math|Vector|MakeVector (Math|Float|Lerp 0.0 2e+01 _alpha) 0.0 0.0) false false)
        (Rendering|Material|SetMaterial (Variables|Default|GetSwitchButtonCombo_Switch1) 2 "/Game/Mesh/Folder/M_EmissiiveGreen.M_EmissiiveGreen"))
      (:Finished
        (Utilities|FlowControl|Sequence
          (:then_0
            (Variables|Default|SetIsActive (Utilities|Select :Index _direction :Forward true :Backward false)))
          (:then_1
            ;[0.2427 0.1562 0.2362] ActorToTriggerLoop
            (for _array_element (Variables|Default|GetInteractables)
              (Utilities|IsValid _array_element
                (:Is%20Valid
                  (if (Utilities|DoesObjectImplementInterface _array_element "/Game/BluePrints/Interfaces/BPI_Trigger.BPI_Trigger_C")
                    (Class|BPITrigger|Trigger(Message) _array_element (Variables|Default|GetIsActive) self))))))
          (:then_2
            (if (Variables|Default|GetPlaySequence)
              ;[0.3552 0.06771 0.06771] PlayLevelSquence
              (Utilities|FlowControl|DoOnce false
                (:Completed
                  (Utilities|IsValid _sequenceplayer
                    (:Is%20Valid
                      (Sequencer|Player|Play _sequenceplayer :!class /Script/MovieScene.MovieSceneSequencePlayer)))))))
          (:then_3
            ;[1 1 1] DisplayText
            (if (Variables|Default|GetDisplayText)
              (if (Variables|Default|GetBlockInputFixeAmount)
                (Variables|Default|SetHowLongToBlockInput (* (Utilities|String|Len (Variables|Default|GetFullText)) (Variables|Default|GetCharactersPerSecond))))
              (if true
                (Input|DisableInput (Game|Player|GetPlayerPawn 0) (Game|GetPlayerController 0))
                (bind _returnvalue_2 (UserInterface|CreateWidget "/Game/UI/WBP_TypewriterPopUp.WBP_TypewriterPopUp_C" 0 (Variables|Default|GetName) (Variables|Default|GetFullText) (Variables|Default|GetCharactersPerSecond) (Variables|Default|GetText%20Should%20Destroyitself%20After%20Display) (+ (Variables|Default|GetHowLongToBlockInput) 2.0) (Variables|Default|GetText%20Finished)))
                (UserInterface|Viewport|AddtoViewport _returnvalue_2 0)
                (Input|DisableInput (Game|Player|GetPlayerPawn 0) (Game|GetPlayerController 0))
                (Utilities|FlowControl|Delay (Variables|Default|GetHowLongToBlockInput))
                (Input|EnableInput (Game|Player|GetPlayerPawn 0) (Game|GetPlayerController 0))
                (Widget|RemovefromParent _returnvalue_2)
                (Input|EnableInput _returnvalue _returnvalue)
                (if (Variables|Default|GetDestroyAfterwards)
                  (Actor|DestroyActor))))))))
    (else
      (Timeline|LeverAnim Reverse))))

(event EventBeginPlay
  ;[1 1 1] Billboard
  (Rendering|SetVisibility (Variables|Default|GetBillboard) false false))

(event EventInteract
  (params (On :type Boolean))
  ;[0.301 0.301 0.301] Animation Lever
  (CallFunction|Interacted))

(fn ConstructionScript)