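; Game mode that runs the main menu, intro, pause, score, death and respawn flow, and directs music.
; BeginPlay creates the game UI and start menu, blends to a cinematic camera and caches the PlayerStart for fade-and-respawn.
; Music and cutscene sounds are FMOD-style 2D events, with timelines crossfading volume parameters and progression events setting LoopRegion to move between sections.
; Some wiring is dead, including the IntroController lookup, and some parameter setters lack names.
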(event Custom|InitMusic
  ;[1 0.2395 0.8775] AudioControl
  ;;[1 1 1] ImHauptMenueAudioAusschaltenBeiStart
  (Class|FMODBlueprintStatics|PlayEvent2D "/Game/FMOD/Events/Music/SingleTracks/HighClean.HighClean")
  (Class|FMODBlueprintStatics|PlayEvent2D "/Game/FMOD/Events/Music/SingleTracks/HighToneDrums.HighToneDrums")
  (Class|FMODBlueprintStatics|PlayEvent2D "/Game/FMOD/Events/Music/SingleTracks/MeloDrums2.MeloDrums2")
  (Class|FMODBlueprintStatics|PlayEvent2D "/Game/FMOD/Events/Music/SingleTracks/HighToneMelody.HighToneMelody")
  (Class|FMODBlueprintStatics|PlayEvent2D "/Game/FMOD/Events/Music/SingleTracks/DeepDrums2.DeepDrums2")
  (CallFunction|AdjustStartMusicVolume))

(event Custom|AdjustStartMusicVolume
  ;[1 1 1] StartMenuVolumeAdjustments
  (Class|FMODBlueprintStatics|SetGlobalParameterbyName "VolumeHighClean" 1.0))

(event Custom|PlayAnimationOnPlayer
  ;[1 1 1] Intro
  (bind _asbp_new_character (Utilities|Casting|CastToBP_NewCharacter (Game|GetPlayerCharacter 0)))
  (Default|PlayIntroAnim _asbp_new_character))

(event Custom|EndIntro
  ;[1 1 1] Intro
  (bind _asabp_character_kt (Utilities|Casting|CastToABP_Character_KT (Components|SkeletalMesh|GetAnimInstance (Variables|/Script/Engine.Character|GetMesh (Game|GetPlayerCharacter 0)))))
  (Default|SetIntroBool _asabp_character_kt))

(event Custom|LoadEnd
  (Game|OpenLevel(byName) "End"))

(event Custom|Benchmark
  ;[1 1 1] Benchmark
  (bind _returnvalue (Settings|GetGameUserSettings))
  (Class|GameUserSettings|RunHardwareBenchmark _returnvalue 10 1.0 1.0)
  (Class|GameUserSettings|ApplyHardwareBenchmarkResults _returnvalue))

(event Custom|StopCutsceneCraneSound
  ;[1 0.2395 0.8775] AudioControl
  ;;[1 1 1] SingleEventStartStop
  (Class|FMODBlueprintStatics|EventInstanceStop (stale Custom|PlayCutsceneCraneSound _returnvalue) false))

(event Custom|OutOfCave
  ;[1 0.2395 0.8775] AudioControl
  ;;[1 1 1] LoopRegionEvents
  ;;;[1 1 1] 1
  (Class|FMODBlueprintStatics|SetGlobalParameterbyName "LoopRegion" 1.5))

(event Custom|PlayCutsceneCraneSound
  ;[1 0.2395 0.8775] AudioControl
  ;;[1 1 1] SingleEventStartStop
  (bind _returnvalue (Class|FMODBlueprintStatics|PlayEvent2D "/Game/FMOD/Events/Environment/SingleSounds/BassWooshCutscene.BassWooshCutscene")))

(event Custom|AddScore
  (params (Value :type Integer))
  ;[1 1 1] AddScore
  (bind _output_get (Variables|Default|SetScore (+ Value (Variables|Default|GetScore))))
  (Default|UpdateScore (Variables|Default|GetGameplayUI) _output_get))

(event Custom|PauseGame
  ;[1 1 1] Pause/UnPause
  (Class|CommonActivatableWidgetContainerBase|AddWidget (Variables|/Game/UI/WBP_GameUI.WBP_GameUI_C|GetPauseStack (Variables|Default|GetGameplayUI)) "/Game/UI/WBP_PauseMenu.WBP_PauseMenu_C")
  (Game|SetGamePaused true)
  (Input|SetInputModeUIOnly (Game|GetPlayerController 0) 0 "DoNotLock" false))

(event Custom|LoopRegionOff
  ;[1 0.2395 0.8775] AudioControl
  ;;[1 1 1] LoopRegionEvents
  (bind _fadeout (Timeline|Timeline_2 PlayFromStart)
    (:Update
      (Class|FMODBlueprintStatics|SetGlobalParameterbyName "LoopRegion" (Math|Float|Lerp 1.0 0.0 _fadeout)))))

(event Custom|CustomEvent
  ;[1 1 1] StartMenuVolumeAdjustments
  (bind _fadeout (Timeline|Timeline_5 PlayFromStart)
    (:Update
      (Class|FMODBlueprintStatics|SetGlobalParameterbyName "VolumeHighClean" (Math|Float|Lerp 0.0 1.0 _fadeout))
      (Class|FMODBlueprintStatics|SetGlobalParameterbyName "HighToneMelodyVolume" (Math|Float|Lerp 1.0 0.0 _fadeout)))))

(event Custom|Creek
  ;[1 0.2395 0.8775] AudioControl
  ;;[1 1 1] LoopRegionEvents
  ;;;[1 1 1] 2
  (Class|FMODBlueprintStatics|SetGlobalParameterbyName "LoopRegion" 2.5))

(event Custom|Booped
  ;[1 1 1] BoopPlayer
)

(event Custom|Cutscene01
  ;[1 0.2395 0.8775] AudioControl
  (bind _fadeout (Timeline|Timeline PlayFromStart)
    (:Update
      (Class|FMODBlueprintStatics|SetGlobalParameterbyName "VolumeHighClean" (Math|Float|Lerp 0.0 1.0 _fadeout))
      (Class|FMODBlueprintStatics|SetGlobalParameterbyName "HighToneMelodyVolume" (Math|Float|Lerp 1.0 0.0 _fadeout)))))

(event Custom|ActivatingElevator
  ;[1 0.2395 0.8775] AudioControl
  ;;[1 1 1] LoopRegionEvents
  ;;;[1 1 1] 3
  (Class|FMODBlueprintStatics|SetGlobalParameterbyName "LoopRegion" 4.5))

(event Custom|ActivatedTheElevator
  ;[1 0.2395 0.8775] AudioControl
  ;;[1 1 1] LoopRegionEvents
  ;;;[1 1 1] 4
  (Class|FMODBlueprintStatics|SetGlobalParameterbyName "LoopRegion" 3.5))

(event Custom|ClearUIOnStart
  (bind _returnvalue (Game|GetPlayerController 0))
  ;[1 1 1] InitializeUI
  (Class|CommonActivatableWidgetContainerBase|ClearWidgets (Variables|/Game/UI/WBP_GameUI.WBP_GameUI_C|GetMainMenuStack (stale Custom|InitUI _returnvalue)))
  (Widget|RemovefromParent (stale Custom|InitUI _returnvalue_2))
  (Input|SetInputModeGameOnly _returnvalue false)
  (Variables|/Script/Engine.PlayerController|SetbShowMouseCursor _returnvalue false))

(event Custom|BlendCameraToPlayer
  (Default|BlendCameratoPlayer (stale Custom|InitUI _returnvalue_3)))

(event Custom|StartCaveMusic
  ;[1 0.2395 0.8775] AudioControl
  (bind _fadeout (Timeline|Timeline_0 PlayFromStart)
    (:Update
      (Class|FMODBlueprintStatics|SetGlobalParameterbyName "VolumeHighClean" (Math|Float|Lerp 1.0 0.0 _fadeout)))))

(event Custom|UnPauseGame
  (bind _returnvalue (Game|GetPlayerController 0))
  ;[1 1 1] Pause/UnPause
  (Class|CommonActivatableWidgetContainerBase|ClearWidgets (Variables|/Game/UI/WBP_GameUI.WBP_GameUI_C|GetPauseStack (Variables|Default|GetGameplayUI)))
  (Game|SetGamePaused false)
  (Input|SetInputModeGameOnly _returnvalue false)
  (Variables|/Script/Engine.PlayerController|SetbShowMouseCursor _returnvalue false))

(event Custom|StartInGameMusic
  ;[1 0.2395 0.8775] AudioControl
  (Class|FMODBlueprintStatics|PlayEvent2D "/Game/FMOD/Events/Music/AllTracks.AllTracks")
  (Class|FMODBlueprintStatics|SetGlobalParameterbyName "LoopRegion" 0.5))

(event Custom|LoopRegionOn
  ;[1 0.2395 0.8775] AudioControl
  ;;[1 1 1] LoopRegionEvents
  (bind _fadeout (Timeline|Timeline_1 PlayFromStart)
    (:Update
      (Class|FMODBlueprintStatics|SetGlobalParameterbyName "LoopRegion" (Math|Float|Lerp 1.0 0.0 _fadeout)))))

(event Custom|InitUI
  ;[1 1 1] InitializeUI
  (if true
    (bind _returnvalue (UserInterface|CreateWidget "/Game/UI/WBP_GameUI.WBP_GameUI_C"))
    (bind _output_get (Variables|Default|SetGameplayUI _returnvalue))
    (UserInterface|Viewport|AddtoViewport _output_get 0)
    (bind _returnvalue_2 (Class|CommonActivatableWidgetContainerBase|AddWidget (Variables|/Game/UI/WBP_GameUI.WBP_GameUI_C|GetMainMenuStack _returnvalue) "/Game/UI/WBP_StartMenuRootV2.WBP_StartMenuRootV2_C"))
    (UserInterface|Viewport|AddtoViewport _returnvalue_2 0)
    (Input|SetInputModeUIOnly (Game|GetPlayerController 0) _returnvalue_2 "DoNotLock" false)
    (bind _returnvalue_3 (Actor|GetActorOfClass "/Game/UI/BP_CineStartCharacter.BP_CineStartCharacter_C"))
    (Default|BlendStartCam _returnvalue_3)))

(event Custom|PlayImpact
  ;[1 0.2395 0.8775] AudioControl
  ;;[1 1 1] SingleEventStartStop
  (Class|FMODBlueprintStatics|PlayEvent2D "/Game/FMOD/Events/Environment/SingleSounds/MetalGateCrash.MetalGateCrash"))

(event Custom|SwitchMainMenuMusic
  ;[1 0.2395 0.8775] AudioControl
  (bind _fadeout (Timeline|Timeline_4 PlayFromStart)
    (:Update
      (Class|FMODBlueprintStatics|SetGlobalParameterbyName "VolumeHighClean" (Math|Float|Lerp 0.0 1.0 _fadeout))
      (Class|FMODBlueprintStatics|SetGlobalParameterbyName "HighToneMelodyVolume" (Math|Float|Lerp 1.0 0.0 _fadeout)))))

(event Custom|StopMusicForPlayStart
  ;[1 0.2395 0.8775] AudioControl
  (bind _newtrack_0 (Timeline|Timeline_3 PlayFromStart)
    (:Update
      (Class|FMODBlueprintStatics|SetGlobalParameterbyName "HighToneMelodyVolume" (Math|Float|Lerp 1.0 0.0 _newtrack_0)))))

(event Custom|PlayerDied
  ;[1 1 1] Death
  (CameraFades|StartCameraFade (Game|GetPlayerCameraManager 0) 0.0 1.0 1.0 "(R=0.000000,G=0.000000,B=0.000000,A=1.000000)" false true)
  (Utilities|FlowControl|Delay 1.0)
  (CallFunction|PlayerSpawn))

(event Custom|PlayerSpawn
  ;[1 1 1] Respawn
  (bind _returnvalue (Game|SpawnActorfromClass "/Game/BluePrints/BP_NewCharacter.BP_NewCharacter_C" (Math|Transform|MakeTransform (.location (Variables|Default|GetPlayerSpawnPoint)) "0, 0, 0" "1.000000,1.000000,1.000000") "Undefined" 0 0))
  (Pawn|Possess (Game|GetPlayerController 0) _returnvalue)
  (CameraFades|StartCameraFade (Game|GetPlayerCameraManager 0) 1.0 0.0 1.0 "(R=0.000000,G=0.000000,B=0.000000,A=1.000000)" false true)
  (bind _asabp_character_kt (Utilities|Casting|CastToABP_Character_KT (Components|SkeletalMesh|GetAnimInstance (Variables|/Script/Engine.Character|GetMesh (Game|GetPlayerCharacter 0)))))
  (Default|SetIntroBoolTrue _asabp_character_kt)
  (Utilities|FlowControl|Delay 0.2)
  (Default|SetIntroBool _asabp_character_kt))

(event Custom|GetPlayerStart
  ;[1 1 1] GetPlayerStart
  (bind _returnvalue (Actor|GetActorOfClass "/Script/Engine.PlayerStart"))
  (Variables|Default|SetPlayerSpawnPoint (Transformation|GetActorTransform _returnvalue)))

(event Custom|SetupInputMode
  ;[1 1 1] EnableInputOnStart
  (Input|SetInputModeGameOnly (Game|GetPlayerController 0) false))

(event Custom|CustomEvent_1
  ;[1 1 1] StartMenuVolumeAdjustments
  (bind _newtrack_0 (Timeline|Timeline_6 PlayFromStart)
    (:Update
      (Class|FMODBlueprintStatics|SetGlobalParameterbyName "HighToneMelodyVolume" (Math|Float|Lerp 1.0 0.0 _newtrack_0)))))

(event Custom|PlayIntro
  ;[1 1 1] Intro
  (Utilities|FlowControl|DoOnce false
    (:Completed
      (bind _asbp_intro_controller (Utilities|Casting|CastToBP_IntroController (Variables|Default|GetIntroController)))
      (Default|PlayIntro _asbp_intro_controller))))

(event EventBeginPlay
  ;[1 1 1] MainMenuInit
  (CallFunction|InitUI)
  (CallFunction|GetPlayerStart)
  (Utilities|FlowControl|Delay 1.0)
  (if (Variables|Default|GetIsIntro)
    (CallFunction|PlayIntro)
    (CallFunction|InitMusic)))

(fn ConstructionScript)