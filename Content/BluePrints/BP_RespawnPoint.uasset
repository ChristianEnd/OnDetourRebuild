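; BP_RespawnPoint is a checkpoint that sets GM_Basic's player spawn point to its SpawnPos location when a BP_NewCharacter overlaps its box.
; The overlap also plays a checkpoint sound and turns the pole's marker material emissive green.
; Optional extra actions send BPI_DeathZone activate or deactivate messages to the Interactable actors and can play a level sequence once.
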(event OnComponentBeginOverlap(Box)
  (params (OverlappedComponent :type Primitive%20Component%20Object%20Reference) (OtherActor :type Actor%20Object%20Reference) (OtherComp :type Primitive%20Component%20Object%20Reference) (OtherBodyIndex :type Integer) (bFromSweep :type Boolean) (SweepResult :type Hit%20Result%20Structure%20%28by%20ref%29))
  (bind _levelsequenceactor (Variables|Default|GetLevelSequenceActor))
  (bind _sequenceplayer (Variables|/Script/LevelSequence.LevelSequenceActor|GetSequencePlayer _levelsequenceactor))
  ;[1 1 1] SettingRespawn
  (Utilities|Casting|CastToBP_NewCharacter OtherActor)
  (bind _asgm_basic (Utilities|Casting|CastToGM_Basic (Game|GetGameMode)))
  (Variables|/Game/BluePrints/GM_Basic.GM_Basic_C|SetPlayerSpawnPoint _asgm_basic (Math|Conversions|ToTransform(Vector) (Transformation|GetWorldLocation (Variables|Default|GetSpawnPos))))
  (Class|FMODBlueprintStatics|PlayEvent2D "/Game/FMOD/Events/Environment/SingleSounds/Checkpoint.Checkpoint")
  ;[1 1 1] VisibilityMarker
  (Rendering|Material|SetMaterial (Variables|Default|GetPole) 1 "/Game/Mesh/Folder/M_EmissiveGreen.M_EmissiveGreen")
  ;[1 1 1] ExtraActions
  (if (Variables|Default|GetExtraActionsNeed)
    (Utilities|FlowControl|Sequence
      (:then_0
        (Variables|Default|SetIsActive (Utilities|Select :Index "Forward" :Forward true :Backward false)))
      (:then_1
        (if (Variables|Default|GetOn/Off)
          ;;[0.2427 0.1562 0.2362] ActorToTriggerLoop
          (for _array_element (Variables|Default|GetInteractable)
            (Utilities|IsValid _array_element
              (:Is%20Valid
                (if (Utilities|DoesObjectImplementInterface _array_element "/Game/BluePrints/Interfaces/BPI_DeathZone.BPI_DeathZone_C")
                  (Class|BPIDeathZone|Activate(Message) _array_element (Variables|Default|GetIsActive) self)))))
          (else
            ;;[1 1 1] OffLoop
            (for _array_element_2 (Variables|Default|GetInteractable)
              (Utilities|IsValid _array_element_2
                (:Is%20Valid
                  (if (Utilities|DoesObjectImplementInterface _array_element_2 "/Game/BluePrints/Interfaces/BPI_DeathZone.BPI_DeathZone_C")
                    (Variables|Default|SetIsActive false)
                    (Class|BPIDeathZone|Activate(Message) _array_element_2 (Variables|Default|GetIsActive) self))))))))
      (:then_2
        (if (Variables|Default|GetPlaySequence)
          ;;[0.3552 0.06771 0.06771] PlayLevelSquence
          (Utilities|FlowControl|DoOnce false
            (:Completed
              (Utilities|IsValid _sequenceplayer
                (:Is%20Valid
                  (Sequencer|Player|Play _sequenceplayer :!class /Script/MovieScene.MovieSceneSequencePlayer))))))))))

(event EventBeginPlay)

(event Collision|EventActorBeginOverlap
  (params (OtherActor :type Actor%20Object%20Reference)))

(event EventTick
  (params (DeltaSeconds :type Float%20%28single-precision%29)))

(fn ConstructionScript)